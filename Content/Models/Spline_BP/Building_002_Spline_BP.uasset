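; Spline-driven building actor that lays mesh segments along a spline and can fade its opacity.
; The construction script adds a spline mesh between each pair of points, matching local positions and tangents, attached under TOPScene.
; It also collects dynamic material instances from each segment's material slots, starting at index 1, into MID.
; FadeIn plays a timeline lerping their Opacity from opaque to transparent, and FadeOut reverses it.
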(event `FadeIn`
  (bind (_direction _ratio) (`Timeline|Fade` :!label _label)
    (:`Update`
      (for _array_element (`self.MID`)
        (`MaterialInstanceDynamic.SetScalarParameterValue` _array_element "Opacity" (`KismetMathLibrary.Lerp` 1.0 0.0 _ratio))))))

(event `FadeOut`
  (goto _label :!via `Reverse`))

(fn `UserConstructionScript`
  (bind _spline (`self.Spline`))
  (for _index (range (+ (- (`SplineComponent.GetNumberOfSplinePoints` (`self.Spline`)) 2) 1))
    (bind _returnvalue (`AddComponent|NODE_AddSplineMeshComponent-0` :`bManualAttachment` true))
    (`|ExecutionSequence`
      (:`then_0`
        (for _index_2 (range 1 (+ (`PrimitiveComponent.GetNumMaterials` _returnvalue) 1))
          (bind _returnvalue_2 (`PrimitiveComponent.CreateDynamicMaterialInstance` _returnvalue _index_2 (`PrimitiveComponent.GetMaterial` _returnvalue _index_2)))
          (`KismetArrayLibrary.Array_Add` (`self.MID`) _returnvalue_2)))
      (:`then_1`
        (`SceneComponent.K2_AttachToComponent` _returnvalue (`self.TOPScene`) "None" "KeepRelative" "KeepRelative" "KeepRelative" true)
        (bind (_location _tangent) (`SplineComponent.GetLocationAndTangentAtSplinePoint` _spline _index "Local"))
        (bind (_location_2 _tangent_2) (`SplineComponent.GetLocationAndTangentAtSplinePoint` _spline (+ _index 1) "Local"))
        (`SplineMeshComponent.SetStartAndEnd` _returnvalue _location _tangent _location_2 _tangent_2 true)))))