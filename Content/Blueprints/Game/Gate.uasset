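; Gate actor that damages Bulby characters touching its KillZone until three Keys open it.
; Capsule overlaps apply damage to a Bulby_BP, or to the BulbyWBP reference on a Base_CBP.
; Each Key entering the same zone sets the next flag, parks above the gate with homing acceleration zeroed and hides an indicator cube.
; The third Key scales KillZone and Stop to zero; any further Key is destroyed.
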(event `self.KillZone.OnComponentBeginOverlap`
  (params (OverlappedComponent :type "PrimitiveComponent Object Reference") (OtherActor :type "Actor Object Reference") (OtherComp :type "PrimitiveComponent Object Reference") (OtherBodyIndex :type Integer) (bFromSweep :type Boolean) (SweepResult :type "HitResult Structure (by ref)"))
  (bind _returnvalue (`self.K2_GetActorLocation`))
  (`|ExecutionSequence`
    (:`then_0`
      (cast `CapsuleComponent` OtherComp)
      (`|ExecutionSequence`
        (:`then_0`
          (bind _asbase_cbp (cast `/Game/Blueprints/PlayableCharacters/Base_CBP` OtherActor))
          (`GameplayStatics.ApplyDamage` (`/Game/Blueprints/PlayableCharacters/Base_CBP.Bulby_WBP` _asbase_cbp) 100.0))
        (:`then_1`
          (bind _asbulby_bp (cast `/Game/Blueprints/PlayableCharacters/Bulby_BP` OtherActor))
          (`GameplayStatics.ApplyDamage` _asbulby_bp 100.0))))
    (:`then_1`
      (bind _askeys (cast `/Game/Blueprints/Game/Keys` OtherActor))
      (if (`self.Key1`)
        (if (`self.Key2`)
          (if (`self.Key3`)
            (`self.K2_DestroyActor` _askeys)
            (else
              (set `self.Key3` true)
              (`self.K2_SetActorLocation` _askeys (+ _returnvalue (-100.0 0.0 100.0)) false false)
              (set `ProjectileMovementComponent.HomingAccelerationMagnitude` 0.0 (`/Game/Blueprints/Game/Keys.ProjectileMovement` _askeys))
              (`SceneComponent.SetRelativeScale3D` (`self.KillZone`) (0.0 0.0 0.0))
              (`SceneComponent.SetRelativeScale3D` (`self.Stop`) (0.0 0.0 0.0))
              (`SceneComponent.SetVisibility` (`self.cube3`) false false)))
          (else
            (set `self.Key2` true)
            (`self.K2_SetActorLocation` _askeys (+ _returnvalue (0.0 0.0 100.0)) false false)
            (set `ProjectileMovementComponent.HomingAccelerationMagnitude` 0.0 (`/Game/Blueprints/Game/Keys.ProjectileMovement` _askeys))
            (`SceneComponent.SetVisibility` (`self.cube2`) false false)))
        (else
          (set `self.Key1` true)
          (`self.K2_SetActorLocation` _askeys (+ _returnvalue (100.0 0.0 100.0)) false false)
          (set `ProjectileMovementComponent.HomingAccelerationMagnitude` 0.0 (`/Game/Blueprints/Game/Keys.ProjectileMovement` _askeys))
          (`SceneComponent.SetVisibility` (`self.Cube`) false false))))))

(fn `UserConstructionScript`)