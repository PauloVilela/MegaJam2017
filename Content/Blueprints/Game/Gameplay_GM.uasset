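; Gameplay game mode that sets up a local multiplayer match when play begins.
; It shows the in-game HUD, then creates local players for the joined count stored in Game_GI.
; Each chosen character spawns at a PlayerStart by index and is possessed by the controller mapped through the saved join order.
; A Bulby actor then spawns at the first PlayerStart.
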(event `self.ReceiveBeginPlay`
  (bind _playerinfo_characterarray (break `/Game/Blueprints/Game/PlayerInfo_Struct` (`self.PlayerInfo`)))
  (bind _outactors (`GameplayStatics.GetAllActorsOfClass` "/Script/Engine.PlayerStart"))
  (set `self.PlayerStarts` _outactors)
  (bind _returnvalue (`|CreateWidget` "/Game/Widgets/Hud/InGameHud_WBP.InGameHud_WBP_C"))
  (bind _output_get (set `self.InGameHud_WBP` _returnvalue))
  (`UserWidget.AddToViewport` _output_get 0)
  (bind _asgame_gi (cast `/Game/Blueprints/Game/Game_GI` (`GameplayStatics.GetGameInstance`)))
  (`|ExecutionSequence`
    (:`then_0`
      (bind _returnvalue_2 (- (`/Game/Blueprints/Game/Game_GI.NumberOfJoinedPlayers` _asgame_gi) 1))
      (for _index (range (+ _returnvalue_2 1))
        ;[1 1 1] Create Controller
        (`GameplayStatics.CreatePlayer` _index))
      ;[1 1 1] SpawnCharacters
      (for _index_2 (range (+ _returnvalue_2 1))
        (bind _returnvalue_3 (`|SpawnActorFromClass` (`|GetArrayItem` _playerinfo_characterarray (`|GetArrayItem` (`/Game/Blueprints/Game/Game_GI.ChosenCharacter` _asgame_gi) _index_2)) (`self.GetTransform` (`|GetArrayItem` (`self.PlayerStarts`) _index_2)) "Undefined" "OverrideRootScale" null null))
        (`Controller.Possess` (`GameplayStatics.GetPlayerController` (`|GetArrayItem` (`/Game/Blueprints/Game/Game_GI.PlayerJoineorderArray` _asgame_gi) _index_2)) _returnvalue_3)))
    (:`then_1`
      ;[1 1 1] Spawn Bulby
      (`|SpawnActorFromClass` "/Game/Blueprints/PlayableCharacters/Bulby_BP.Bulby_BP_C" (`self.GetTransform` (`|GetArrayItem` (`self.PlayerStarts`))) "AlwaysSpawn" "OverrideRootScale" null null))))

(fn `UserConstructionScript`)