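; Checkpoint actor that registers itself as the current checkpoint when a Base_CBP character enters its radius.
; On BeginPlay it finds the CheckPointManager_BP in the level.
; Overlap sends its location and self reference to the manager and turns on its lamp post light.
; A DeactivateCheckpoint event switches that light off.
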(event `self.ReceiveBeginPlay`
  ;[1 1 1] Retreive Checkpoint manager in scene
  (bind _outactors (`GameplayStatics.GetAllActorsOfClass` "/Game/Blueprints/Game/CheckPointManager_BP.CheckPointManager_BP_C"))
  (for _array_element _outactors
    (set `self.CheckPointManager_BP` _array_element)))

(event `self.CheckPointRadius.OnComponentBeginOverlap`
  (params (OverlappedComponent :type "PrimitiveComponent Object Reference") (OtherActor :type "Actor Object Reference") (OtherComp :type "PrimitiveComponent Object Reference") (OtherBodyIndex :type Integer) (bFromSweep :type Boolean) (SweepResult :type "HitResult Structure (by ref)"))
  ;[1 1 1] Activate Checkpoint
  (cast `/Game/Blueprints/PlayableCharacters/Base_CBP` OtherActor)
  (`/Game/Blueprints/Game/CheckPointManager_BP.UpdatedCurrentLocation` (`self.CheckPointManager_BP`) (`self.K2_GetActorLocation`) self)
  (`SceneComponent.SetVisibility` (`self.LampPostLight`) true false))

(event `DeactivateCheckpoint`
  ;[1 1 1] Deactivate Checkpoint
  (`SceneComponent.SetVisibility` (`self.LampPostLight`) false false))

(fn `UserConstructionScript`)