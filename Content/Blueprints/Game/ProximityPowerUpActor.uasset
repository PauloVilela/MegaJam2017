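; ProximityPowerUpActor is a placed actor that triggers a proximity-based power-up on Base_CBP characters that come within its range.
; Overlapping its MaxRange sphere calls StartPowerUp on the character's BulbyWBP widget, passing the influence range and actor location.
; Leaving the sphere calls EndPowerUp on that widget.
; The construction script derives the sphere radius from half the Y value of MyInfluenceRange.
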(event `self.MaxRange.OnComponentBeginOverlap`
  (params (OverlappedComponent :type "PrimitiveComponent Object Reference") (OtherActor :type "Actor Object Reference") (OtherComp :type "PrimitiveComponent Object Reference") (OtherBodyIndex :type Integer) (bFromSweep :type Boolean) (SweepResult :type "HitResult Structure (by ref)"))
  (bind _asbase_cbp (cast `/Game/Blueprints/PlayableCharacters/Base_CBP` OtherActor))
  (`/Game/Blueprints/PlayableCharacters/Bulby_BP.StartPowerUp` (`/Game/Blueprints/PlayableCharacters/Base_CBP.Bulby_WBP` _asbase_cbp) (`self.MyInfluenceRange`) (`self.K2_GetActorLocation`)))

(event `self.MaxRange.OnComponentEndOverlap`
  (params (OverlappedComponent :type "PrimitiveComponent Object Reference") (OtherActor :type "Actor Object Reference") (OtherComp :type "PrimitiveComponent Object Reference") (OtherBodyIndex :type Integer))
  (bind _asbase_cbp (cast `/Game/Blueprints/PlayableCharacters/Base_CBP` OtherActor))
  (`/Game/Blueprints/PlayableCharacters/Bulby_BP.EndPowerUp` (`/Game/Blueprints/PlayableCharacters/Base_CBP.Bulby_WBP` _asbase_cbp)))

(fn `UserConstructionScript`
  (bind (_myinfluencerange_x _myinfluencerange_y) (`KismetMathLibrary.BreakVector2D` (`self.MyInfluenceRange`)))
  (`SphereComponent.SetSphereRadius` (`self.MaxRange`) (/ _myinfluencerange_y 2.0) true))