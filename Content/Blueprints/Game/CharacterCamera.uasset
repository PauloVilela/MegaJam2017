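; Follow camera actor that trails its target's MidPoint at an offset, snapping there on the first tick.
; Each tick it moves toward that ideal location under per-axis and total speed caps, with distance-banded SpeedAdjusters scaling the total cap.
; Radius and per-axis clipping add uncapped movement for any lag beyond the distance limits.
; Rotation is computed from the ideal location, so lag does not change the viewing angle.
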(event `self.ReceiveTick`
  (params (DeltaSeconds :type "Float (single-precision)"))
  (bind _deltalocation (`self.DeltaLocation`))
  (bind _cameradistancelimiter (`self.CameraDistanceLimiter`))
  (bind (_deltalocation_x _deltalocation_y _deltalocation_z) (`KismetMathLibrary.BreakVector` (`self.DeltaLocation`)))
  (bind (_deltalocation_x_2 _deltalocation_y_2 _deltalocation_z_2) (`KismetMathLibrary.BreakVector` (`self.DeltaLocation`)))
  (bind (_movementthisframeduetocap_x _movementthisframeduetocap_y) (`KismetMathLibrary.BreakVector` (`self.MovementThisFrameDueToCap`)))
  (bind (_deltalocation_x_3 _deltalocation_y_3 _deltalocation_z_3) (`KismetMathLibrary.BreakVector` (`self.DeltaLocation`)))
  (bind (_deltalocation_x_4 _deltalocation_y_4 _deltalocation_z_4) (`KismetMathLibrary.BreakVector` (`self.DeltaLocation`)))
  (bind (_cameradistancelimiterperaxis_x _cameradistancelimiterperaxis_y _cameradistancelimiterperaxis_z) (`KismetMathLibrary.BreakVector` (`self.CameraDistanceLimiterPerAxis`)))
  (bind (_cameradistancelimiterperaxis_x_2 _cameradistancelimiterperaxis_y_2 _cameradistancelimiterperaxis_z_2) (`KismetMathLibrary.BreakVector` (`self.CameraDistanceLimiterPerAxis`)))
  (bind (_deltalocation_x_5 _deltalocation_y_5) (`KismetMathLibrary.BreakVector` (`self.DeltaLocation`)))
  (bind (_deltalocation_x_6 _deltalocation_y_6) (`KismetMathLibrary.BreakVector` (`self.DeltaLocation`)))
  (bind (_movementthisframeduetocap_x_2 _movementthisframeduetocap_y_2 _movementthisframeduetocap_z) (`KismetMathLibrary.BreakVector` (`self.MovementThisFrameDueToCap`)))
  (bind (_deltalocation_x_7 _deltalocation_y_7) (`KismetMathLibrary.BreakVector` (`self.DeltaLocation`)))
  (bind (_deltalocation_x_8 _deltalocation_y_8 _deltalocation_z_5) (`KismetMathLibrary.BreakVector` (`self.DeltaLocation`)))
  (bind (_cameradistancelimiterperaxis_x_3 _cameradistancelimiterperaxis_y_3) (`KismetMathLibrary.BreakVector` (`self.CameraDistanceLimiterPerAxis`)))
  (bind (_cameradistancelimiterperaxis_x_4 _cameradistancelimiterperaxis_y_4) (`KismetMathLibrary.BreakVector` (`self.CameraDistanceLimiterPerAxis`)))
  (bind _deltalocation_x_9 (`KismetMathLibrary.BreakVector` (`self.DeltaLocation`)))
  (bind _deltalocation_x_10 (`KismetMathLibrary.BreakVector` (`self.DeltaLocation`)))
  (bind (_movementthisframeduetocap_x_3 _movementthisframeduetocap_y_3 _movementthisframeduetocap_z_2) (`KismetMathLibrary.BreakVector` (`self.MovementThisFrameDueToCap`)))
  (bind _deltalocation_x_11 (`KismetMathLibrary.BreakVector` (`self.DeltaLocation`)))
  (bind (_deltalocation_x_12 _deltalocation_y_9 _deltalocation_z_6) (`KismetMathLibrary.BreakVector` (`self.DeltaLocation`)))
  (bind _cameradistancelimiterperaxis_x_5 (`KismetMathLibrary.BreakVector` (`self.CameraDistanceLimiterPerAxis`)))
  (bind _cameradistancelimiterperaxis_x_6 (`KismetMathLibrary.BreakVector` (`self.CameraDistanceLimiterPerAxis`)))
  (bind (_cameradistancelimiterperaxis_x_7 _cameradistancelimiterperaxis_y_5 _cameradistancelimiterperaxis_z_3) (`KismetMathLibrary.BreakVector` (`self.CameraDistanceLimiterPerAxis`)))
  (bind (_deltalocation_x_13 _deltalocation_y_10 _deltalocation_z_7) (`KismetMathLibrary.BreakVector` (`self.DeltaLocation`)))
  (bind (_deltalocation_x_14 _deltalocation_y_11 _deltalocation_z_8) (`KismetMathLibrary.BreakVector` (`self.DeltaLocation`)))
  (bind (_maxmovementthisframe_peraxis_x _maxmovementthisframe_peraxis_y _maxmovementthisframe_peraxis_z) (`KismetMathLibrary.BreakVector` (`self.MaxMovementThisFrame_PerAxis`)))
  (bind (_deltalocation_x_15 _deltalocation_y_12 _deltalocation_z_9) (`KismetMathLibrary.BreakVector` (`self.DeltaLocation`)))
  (bind _returnvalue (`KismetMathLibrary.VSize` _deltalocation))
  (bind _returnvalue_2 (`KismetMathLibrary.VSize` (`self.DeltaLocation`)))
  (bind _midpoint (`/Game/Blueprints/PlayableCharacters/Bulby_BP.MidPoint` (`self.MyTargetToFollow`)))
  (`|ExecutionSequence`
    (:`then_0`
      ;[1 1 1] Quick Fix for initial location
      (`/Engine/EditorBlueprintResources/StandardMacros.DoOnce` false
        (:`Completed`
          (`self.K2_SetActorLocation` (+ (`self.IdealOffset`) (`/Game/Blueprints/PlayableCharacters/Bulby_BP.MidPoint` (`self.MyTargetToFollow`)))))))
    (:`then_1`
      (`|ExecutionSequence`
        (:`then_0`
          (set `self.IdealLocation` (+ (`/Game/Blueprints/PlayableCharacters/Bulby_BP.MidPoint` (`self.MyTargetToFollow`)) (`self.IdealOffset`)))
          (set `self.CurrentLocation` (`self.K2_GetActorLocation`))
          (set `self.DeltaLocation` (- (`self.IdealLocation`) (`self.CurrentLocation`)))
          (set `self.MaxMovementThisFrame_PerAxis` (* (`self.CameraSpeedPerAxis`) (`GameplayStatics.GetWorldDeltaSeconds`)))
          (set `self.MovementThisFrameDueToCap` (0.0 0.0 0.0))
          (set `self.CurrentSpeedLimiter` (`self.CameraSpeedLimiter`))
          (`|ExecutionSequence`
            (:`then_0`
              (if (> _returnvalue _cameradistancelimiter)
                (set `self.CapVector` (* (`KismetMathLibrary.Normal` _deltalocation) (- _returnvalue _cameradistancelimiter)))
                (set `self.MovementThisFrameDueToCap` (+ (`self.CapVector`) (`self.MovementThisFrameDueToCap`)))
                (set `self.DeltaLocation` (- (`self.DeltaLocation`) (`self.CapVector`)))))
            (:`then_1`
              (`|ExecutionSequence`
                (:`then_0`
                  (if (> (`KismetMathLibrary.Abs` _deltalocation_x_13) _cameradistancelimiterperaxis_x_7)
                    (set `self.MovementThisFrameDueToCap` (`KismetMathLibrary.MakeVector` (* (`KismetMathLibrary.SignOfFloat` _deltalocation_x_9) (- (`KismetMathLibrary.Abs` _deltalocation_x_11) _cameradistancelimiterperaxis_x_6)) _movementthisframeduetocap_y_3 _movementthisframeduetocap_z_2))
                    (set `self.DeltaLocation` (`KismetMathLibrary.MakeVector` (+ _deltalocation_x_10 (`KismetMathLibrary.FClamp` _deltalocation_x_12 (* _cameradistancelimiterperaxis_x_5 -1.0) _cameradistancelimiterperaxis_x_5)) _deltalocation_y_9 _deltalocation_z_6))))
                (:`then_1`
                  (if (> (`KismetMathLibrary.Abs` _deltalocation_y_10) _cameradistancelimiterperaxis_y_5)
                    (set `self.MovementThisFrameDueToCap` (`KismetMathLibrary.MakeVector` _movementthisframeduetocap_x_2 (* (`KismetMathLibrary.SignOfFloat` _deltalocation_y_5) (- (`KismetMathLibrary.Abs` _deltalocation_y_7) _cameradistancelimiterperaxis_y_4)) _movementthisframeduetocap_z))
                    (set `self.DeltaLocation` (`KismetMathLibrary.MakeVector` _deltalocation_x_8 (+ _deltalocation_y_6 (`KismetMathLibrary.FClamp` _deltalocation_y_8 (* _cameradistancelimiterperaxis_y_3 -1.0) _cameradistancelimiterperaxis_y_3)) _deltalocation_z_5))))
                (:`then_2`
                  (if (> (`KismetMathLibrary.Abs` _deltalocation_z_7) _cameradistancelimiterperaxis_z_3)
                    (set `self.MovementThisFrameDueToCap` (`KismetMathLibrary.MakeVector` _movementthisframeduetocap_x _movementthisframeduetocap_y (* (`KismetMathLibrary.SignOfFloat` _deltalocation_z) (- (`KismetMathLibrary.Abs` _deltalocation_z_3) _cameradistancelimiterperaxis_z))))
                    (set `self.DeltaLocation` (`KismetMathLibrary.MakeVector` _deltalocation_x_4 _deltalocation_y_4 (+ _deltalocation_z_2 (`KismetMathLibrary.FClamp` _deltalocation_z_4 (* _cameradistancelimiterperaxis_z_2 -1.0) _cameradistancelimiterperaxis_z_2))))))))
            (:`then_2`
              (for _array_element (`self.SpeedAdjusters`)
                (bind (_distancerange _speedmultiplierrange) (break `/Game/Blueprints/Game/ChaseCamSpeedAdjustment` _array_element))
                (bind (_x _y) (`KismetMathLibrary.BreakVector2D` _distancerange))
                (if (== _returnvalue_2 (`KismetMathLibrary.FClamp` _returnvalue_2 _x _y))
                  (bind (_x_2 _y_2) (`KismetMathLibrary.BreakVector2D` _distancerange))
                  (bind (_x_3 _y_3) (`KismetMathLibrary.BreakVector2D` _speedmultiplierrange))
                  (set `self.CurrentSpeedLimiter` (* (`self.CurrentSpeedLimiter`) (`KismetMathLibrary.MapRangeUnclamped` (`KismetMathLibrary.VSize` (`self.DeltaLocation`)) _x_2 _y_2 _x_3 _y_3)))
                  (break))))
            (:`then_3`
              (set `self.DesiredMovementThisFrame` (`KismetMathLibrary.MakeVector` (`KismetMathLibrary.FMin` (`KismetMathLibrary.Abs` _deltalocation_x_14) (* _maxmovementthisframe_peraxis_x (`KismetMathLibrary.SignOfFloat` _deltalocation_x_15))) (`KismetMathLibrary.FMin` (`KismetMathLibrary.Abs` _deltalocation_y_11) (* _maxmovementthisframe_peraxis_y (`KismetMathLibrary.SignOfFloat` _deltalocation_y_12))) (`KismetMathLibrary.FMin` (`KismetMathLibrary.Abs` _deltalocation_z_8) (* _maxmovementthisframe_peraxis_z (`KismetMathLibrary.SignOfFloat` _deltalocation_z_9)))))
              (set `self.DesiredMovementThisFrame` (`KismetMathLibrary.ClampVectorSize` (`self.DesiredMovementThisFrame`) 0.0 (* (`self.CurrentSpeedLimiter`) (`GameplayStatics.GetWorldDeltaSeconds`)))))))
        (:`then_1`
          (`self.K2_SetActorLocation` (+ (`self.CurrentLocation`) (`self.DesiredMovementThisFrame`) (`self.MovementThisFrameDueToCap`)))
          (`self.K2_SetActorRotation` (`KismetMathLibrary.FindLookAtRotation` (+ (`self.IdealOffset`) _midpoint) _midpoint)))))))

(fn `UserConstructionScript`)