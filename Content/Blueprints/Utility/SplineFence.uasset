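; SplineFence is a fence actor that builds itself along its spline in the construction script using spline mesh components.
; It places a start mesh, repeated middle meshes and an end mesh, spaced by per-piece approximate sizes, with normalized tangents scaled to those sizes.
; The middle count is floored from the full spline length, ignoring cap sizes.
; Points are world-space minus actor location, so actor rotation and scale are not compensated.
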(fn `UserConstructionScript`
  (bind _returnvalue (`self.K2_GetActorLocation`))
  (bind _returnvalue_2 (`self.K2_GetActorLocation`))
  (bind _returnvalue_3 (`self.K2_GetActorLocation`))
  (bind _spline (`self.Spline`))
  (bind _approximativesizestart (`self.ApproximativeSizeStart`))
  (bind _approximativesize (`self.ApproximativeSize`))
  (bind _approximativesizeend (`self.ApproximativeSizeEnd`))
  (bind _spline_2 (`self.Spline`))
  (bind _spline_3 (`self.Spline`))
  (bind _approximativesizestart_2 (`self.ApproximativeSizeStart`))
  (bind _returnvalue_4 (+ (`self.ApproximativeSizeStart`) (* (`KismetMathLibrary.FFloor` (/ (`SplineComponent.GetSplineLength` (`self.Spline`)) (`self.ApproximativeSize`))) (`self.ApproximativeSize`))))
  (bind _returnvalue_5 (+ _returnvalue_4 _approximativesizeend))
  (`|ExecutionSequence`
    (:`then_0`
      (bind _returnvalue_6 (`AddComponent|NODE_AddSplineMeshComponent-0`))
      (`StaticMeshComponent.SetStaticMesh` _returnvalue_6 (`self.MeshStart`))
      (`SplineMeshComponent.SetStartAndEnd` _returnvalue_6 (- (`SplineComponent.GetLocationAtDistanceAlongSpline` _spline_3 0.0 "World") _returnvalue_3) (* (`KismetMathLibrary.Normal` (`SplineComponent.GetTangentAtDistanceAlongSpline` _spline_3 0.0 "World")) _approximativesizestart_2) (- (`SplineComponent.GetLocationAtDistanceAlongSpline` _spline_3 _approximativesizestart_2 "World") _returnvalue_3) (* (`KismetMathLibrary.Normal` (`SplineComponent.GetTangentAtDistanceAlongSpline` _spline_3 _approximativesizestart_2 "World")) _approximativesizestart_2) true))
    (:`then_1`
      (for _index (range (`KismetMathLibrary.FFloor` (/ (`SplineComponent.GetSplineLength` (`self.Spline`)) (`self.ApproximativeSize`))))
        (bind _returnvalue_7 (`AddComponent|NODE_AddSplineMeshComponent-1`))
        (`StaticMeshComponent.SetStaticMesh` _returnvalue_7 (`self.Mesh`))
        (bind _returnvalue_8 (+ (* _index _approximativesize) _approximativesizestart))
        (bind _returnvalue_9 (+ (* (+ _index 1) _approximativesize) _approximativesizestart))
        (`SplineMeshComponent.SetStartAndEnd` _returnvalue_7 (- (`SplineComponent.GetLocationAtDistanceAlongSpline` _spline_2 _returnvalue_8 "World") _returnvalue) (* (`KismetMathLibrary.Normal` (`SplineComponent.GetTangentAtDistanceAlongSpline` _spline_2 _returnvalue_8 "World")) _approximativesize) (- (`SplineComponent.GetLocationAtDistanceAlongSpline` _spline_2 _returnvalue_9 "World") _returnvalue) (* (`KismetMathLibrary.Normal` (`SplineComponent.GetTangentAtDistanceAlongSpline` _spline_2 _returnvalue_9 "World")) _approximativesize) true)))
    (:`then_2`
      (bind _returnvalue_10 (`AddComponent|NODE_AddSplineMeshComponent-3`))
      (`StaticMeshComponent.SetStaticMesh` _returnvalue_10 (`self.MeshEnd`))
      (`SplineMeshComponent.SetStartAndEnd` _returnvalue_10 (- (`SplineComponent.GetLocationAtDistanceAlongSpline` _spline _returnvalue_4 "World") _returnvalue_2) (* (`KismetMathLibrary.Normal` (`SplineComponent.GetTangentAtDistanceAlongSpline` _spline _returnvalue_4 "World")) _approximativesizeend) (- (`SplineComponent.GetLocationAtDistanceAlongSpline` _spline _returnvalue_5 "World") _returnvalue_2) (* (`KismetMathLibrary.Normal` (`SplineComponent.GetTangentAtDistanceAlongSpline` _spline _returnvalue_5 "World")) _approximativesizeend) true))))