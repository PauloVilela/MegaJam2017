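; Bulby is the players' light companion, hovering at their midpoint with capped, distance-scaled speed and publishing its XY to a material parameter collection.
; Its health drains gradually above a threshold, and damage resizes the safe-zone sphere and spotlight cone, which separate light from darkness for players.
; At zero health, it refills and teleports everyone to the checkpoint.
; It also spawns the shared camera and computes a proximity power-up value.
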(event `self.ReceiveBeginPlay`
  ;[1 1 1] Begin Play
  (bind _outactors (`GameplayStatics.GetAllActorsOfClass` "/Game/Blueprints/PlayableCharacters/Base_CBP.Base_CBP_C"))
  (bind _output_get (set `self.MyFriend` _outactors))
  (if (not (> 2 (`KismetArrayLibrary.Array_Length` _output_get)))
    (set `self.SinglePlayerGame` false))
  (bind _returnvalue (`|SpawnActorFromClass` "/Game/Blueprints/Game/CharacterCamera.CharacterCamera_C" (`KismetMathLibrary.MakeTransform` (0.0 0.0 0.0)) "AlwaysSpawn" "OverrideRootScale" null null))
  (`|ExecutionSequence`
    (:`then_0`
      (bind _output_get_2 (set `/Game/Blueprints/Game/CharacterCamera.MyTargetToFollow` self _returnvalue))
      (`self.AddTickPrerequisiteActor` _output_get_2 self))
    (:`then_1`
      (for (_array_element _array_index) _output_get
        (`PlayerController.SetViewTargetWithBlend` (`GameplayStatics.GetPlayerController` _array_element _array_index) _returnvalue 0.0 "VTBlend_Linear" 0.0 false)
        (set `/Game/Blueprints/PlayableCharacters/Base_CBP.Bulby_WBP` self _array_element)))
    (:`then_2`
      (bind _foundwidgets (`WidgetBlueprintLibrary.GetAllWidgetsOfClass` "/Game/Widgets/Hud/InGameHud_WBP.InGameHud_WBP_C"))
      (for _array_element_2 _foundwidgets
        (bind _output_get_3 (set `self.InGameHud_WBP` _array_element_2))
        (`/Game/Widgets/Hud/InGameHud_WBP.Get MaxHealth` _output_get_3 (`self.BulbyMaxHealth`))))
    (:`then_3`
      (bind _outactors_2 (`GameplayStatics.GetAllActorsOfClass` "/Game/Blueprints/Game/CheckPointManager_BP.CheckPointManager_BP_C"))
      (for _array_element_3 _outactors_2
        (set `self.CheckPointManager_BP` _array_element_3)))))

(event `Damage Tick`
  ;[1 1 1] Darkness Damage over time
  (if (>= (`self.BulbyHealth`) 40.0)
    (`KismetSystemLibrary.Delay` 1.0)
    (`GameplayStatics.ApplyDamage` self 1.0) ; Darkness Damage
  ))

(event `self.SafeZone.OnComponentEndOverlap`
  (params (OverlappedComponent :type "PrimitiveComponent Object Reference") (OtherActor :type "Actor Object Reference") (OtherComp :type "PrimitiveComponent Object Reference") (OtherBodyIndex :type Integer))
  ;[1 1 1] Take Damage Outside Radius
  (bind _asbase_cbp (cast `/Game/Blueprints/PlayableCharacters/Base_CBP` OtherActor))
  (`/Game/Blueprints/PlayableCharacters/Base_CBP.Into Darkness` _asbase_cbp))

(event `Set Safe Zone Radius`
  (bind (_safezoneradius_x _safezoneradius_y) (`KismetMathLibrary.BreakVector2D` (`self.SafeZoneRadius`)))
  (bind (_safezoneradius_x_2 _safezoneradius_y_2) (`KismetMathLibrary.BreakVector2D` (`self.SafeZoneRadius`)))
  (bind (_safezonerange_x _safezonerange_y) (`KismetMathLibrary.BreakVector2D` (`self.SafeZoneRange`)))
  (bind _safezonedesiredradius (`self.SafeZoneDesiredRadius`))
  (bind _spotlight (`self.SpotLight`))
  (set `self.SafeZoneCurrentRadius` (`self.SafeZoneTransitionRadius`))
  (set `self.SafeZoneDesiredRadius` (`KismetMathLibrary.MapRangeClamped` (`self.BulbyHealth`) _safezonerange_x _safezonerange_y _safezoneradius_x_2 _safezoneradius_y_2))
  (bind (_direction _lerp) (`Timeline|SafeZoneRadiusTL` :!via `PlayFromStart`)
    (:`Update`
      (bind _returnvalue (`KismetMathLibrary.Lerp` (`self.SafeZoneCurrentRadius`) _safezonedesiredradius _lerp))
      (set `self.SafeZoneTransitionRadius` _returnvalue)
      (`SphereComponent.SetSphereRadius` (`self.SafeZone`) _returnvalue true)
      (bind _returnvalue_2 (`KismetMathLibrary.MapRangeClamped` _returnvalue _safezoneradius_x _safezoneradius_y 55.0 75.0))
      (`SpotLightComponent.SetOuterConeAngle` _spotlight _returnvalue_2)
      (`SpotLightComponent.SetInnerConeAngle` _spotlight (- _returnvalue_2 5.0)))
    (:`Finished`
      (set `self.SafeZoneCurrentRadius` _safezonedesiredradius))))

(event `self.SafeZone.OnComponentBeginOverlap`
  (params (OverlappedComponent :type "PrimitiveComponent Object Reference") (OtherActor :type "Actor Object Reference") (OtherComp :type "PrimitiveComponent Object Reference") (OtherBodyIndex :type Integer) (bFromSweep :type Boolean) (SweepResult :type "HitResult Structure (by ref)"))
  ;[1 1 1] Take Damage Outside Radius
  (bind _asbase_cbp (cast `/Game/Blueprints/PlayableCharacters/Base_CBP` OtherActor))
  (`/Game/Blueprints/PlayableCharacters/Base_CBP.Into Light` _asbase_cbp))

(event `self.ReceiveAnyDamage`
  (params (Damage :type "Float (single-precision)") (DamageType :type "DamageType Object Reference") (InstigatedBy :type "Controller Object Reference") (DamageCauser :type "Actor Object Reference"))
  (bind _bulbymaxhealth (`self.BulbyMaxHealth`))
  (bind _currentcheckpointloc (`/Game/Blueprints/Game/CheckPointManager_BP.CurrentCheckpointLoc` (`self.CheckPointManager_BP`)))
  ;[1 1 1] Take Damage
  (`|ExecutionSequence`
    (:`then_0`
      (set `self.BulbyHealth` (`KismetMathLibrary.FClamp` (- (`self.BulbyHealth`) Damage) 0.0 (`self.BulbyMaxHealth`)))
      (`self.Set Safe Zone Radius`)
      (`/Game/Widgets/Hud/InGameHud_WBP.UpdatedHealth` (`self.InGameHud_WBP`) (`self.BulbyHealth`)))
    (:`then_1`
      (if (== (`self.BulbyHealth`) 0.0)
        (set `self.BulbyHealth` _bulbymaxhealth)
        (`self.Set Safe Zone Radius`)
        (`/Game/Widgets/Hud/InGameHud_WBP.Get MaxHealth` (`self.InGameHud_WBP`) _bulbymaxhealth)
        (`self.K2_SetActorLocation` _currentcheckpointloc)
        (for _array_element (`self.MyFriend`)
          (`self.K2_SetActorLocation` _array_element (`KismetMathLibrary.RandomPointInBoundingBox` (`KismetMathLibrary.MakeVector` (.x _currentcheckpointloc) (.y _currentcheckpointloc) (+ (.z _currentcheckpointloc) (`CapsuleComponent.CapsuleHalfHeight` (`Character.CapsuleComponent` _array_element)))) (250.0 250.0 0.0)) false false))))))

(event `StartPowerUp`
  (params (PowerUpRange :type "Vector2D Structure") (Location :type "Vector Structure"))
  (bind (_x _y) (`KismetMathLibrary.BreakVector2D` PowerUpRange))
  (goto _label :!via `Open`))

(event `EndPowerUp`
  (goto _label :!via `Close`))

(event `self.ReceiveTick`
  (params (DeltaSeconds :type "Float (single-precision)"))
  (bind _deltalocation (`self.DeltaLocation`))
  (bind _bulbydistancelimiter (`self.BulbyDistanceLimiter`))
  (bind (_deltalocation_x _deltalocation_y _deltalocation_z) (`KismetMathLibrary.BreakVector` (`self.DeltaLocation`)))
  (bind (_deltalocation_x_2 _deltalocation_y_2 _deltalocation_z_2) (`KismetMathLibrary.BreakVector` (`self.DeltaLocation`)))
  (bind (_movementthisframeduetocap_x _movementthisframeduetocap_y) (`KismetMathLibrary.BreakVector` (`self.MovementThisFrameDueToCap`)))
  (bind (_deltalocation_x_3 _deltalocation_y_3 _deltalocation_z_3) (`KismetMathLibrary.BreakVector` (`self.DeltaLocation`)))
  (bind (_deltalocation_x_4 _deltalocation_y_4 _deltalocation_z_4) (`KismetMathLibrary.BreakVector` (`self.DeltaLocation`)))
  (bind (_bulbydistancelimiterperaxis_x _bulbydistancelimiterperaxis_y _bulbydistancelimiterperaxis_z) (`KismetMathLibrary.BreakVector` (`self.BulbyDistanceLimiterPerAxis`)))
  (bind (_bulbydistancelimiterperaxis_x_2 _bulbydistancelimiterperaxis_y_2 _bulbydistancelimiterperaxis_z_2) (`KismetMathLibrary.BreakVector` (`self.BulbyDistanceLimiterPerAxis`)))
  (bind (_deltalocation_x_5 _deltalocation_y_5) (`KismetMathLibrary.BreakVector` (`self.DeltaLocation`)))
  (bind (_deltalocation_x_6 _deltalocation_y_6) (`KismetMathLibrary.BreakVector` (`self.DeltaLocation`)))
  (bind (_movementthisframeduetocap_x_2 _movementthisframeduetocap_y_2 _movementthisframeduetocap_z) (`KismetMathLibrary.BreakVector` (`self.MovementThisFrameDueToCap`)))
  (bind (_deltalocation_x_7 _deltalocation_y_7) (`KismetMathLibrary.BreakVector` (`self.DeltaLocation`)))
  (bind (_deltalocation_x_8 _deltalocation_y_8 _deltalocation_z_5) (`KismetMathLibrary.BreakVector` (`self.DeltaLocation`)))
  (bind (_bulbydistancelimiterperaxis_x_3 _bulbydistancelimiterperaxis_y_3) (`KismetMathLibrary.BreakVector` (`self.BulbyDistanceLimiterPerAxis`)))
  (bind (_bulbydistancelimiterperaxis_x_4 _bulbydistancelimiterperaxis_y_4) (`KismetMathLibrary.BreakVector` (`self.BulbyDistanceLimiterPerAxis`)))
  (bind _deltalocation_x_9 (`KismetMathLibrary.BreakVector` (`self.DeltaLocation`)))
  (bind _deltalocation_x_10 (`KismetMathLibrary.BreakVector` (`self.DeltaLocation`)))
  (bind (_movementthisframeduetocap_x_3 _movementthisframeduetocap_y_3 _movementthisframeduetocap_z_2) (`KismetMathLibrary.BreakVector` (`self.MovementThisFrameDueToCap`)))
  (bind _deltalocation_x_11 (`KismetMathLibrary.BreakVector` (`self.DeltaLocation`)))
  (bind (_deltalocation_x_12 _deltalocation_y_9 _deltalocation_z_6) (`KismetMathLibrary.BreakVector` (`self.DeltaLocation`)))
  (bind _bulbydistancelimiterperaxis_x_5 (`KismetMathLibrary.BreakVector` (`self.BulbyDistanceLimiterPerAxis`)))
  (bind _bulbydistancelimiterperaxis_x_6 (`KismetMathLibrary.BreakVector` (`self.BulbyDistanceLimiterPerAxis`)))
  (bind (_bulbydistancelimiterperaxis_x_7 _bulbydistancelimiterperaxis_y_5 _bulbydistancelimiterperaxis_z_3) (`KismetMathLibrary.BreakVector` (`self.BulbyDistanceLimiterPerAxis`)))
  (bind (_deltalocation_x_13 _deltalocation_y_10 _deltalocation_z_7) (`KismetMathLibrary.BreakVector` (`self.DeltaLocation`)))
  (bind _myfriend (`self.MyFriend`))
  (bind (_proximitypoweruprange_x _proximitypoweruprange_y) (`KismetMathLibrary.BreakVector2D` (`self.ProximityPowerUpRange`)))
  (bind (_deltalocation_x_14 _deltalocation_y_11 _deltalocation_z_8) (`KismetMathLibrary.BreakVector` (`self.DeltaLocation`)))
  (bind (_maxmovementthisframe_peraxis_x _maxmovementthisframe_peraxis_y _maxmovementthisframe_peraxis_z) (`KismetMathLibrary.BreakVector` (`self.MaxMovementThisFrame_PerAxis`)))
  (bind (_deltalocation_x_15 _deltalocation_y_12 _deltalocation_z_9) (`KismetMathLibrary.BreakVector` (`self.DeltaLocation`)))
  (bind _returnvalue (`KismetMathLibrary.VSize` _deltalocation))
  (bind _returnvalue_2 (`KismetMathLibrary.VSize` (`self.DeltaLocation`)))
  (`|ExecutionSequence`
    (:`then_0`
      (`self.MidPointLocation`)
      (if (`self.SinglePlayerGame`)
        (`/Engine/EditorBlueprintResources/StandardMacros.Gate` true :!label _label
          (:`Exit`
            (set `self.ProximityPowerUp` (`KismetMathLibrary.VSize` (- (`self.K2_GetActorLocation` (`|GetArrayItem` (`self.MyFriend`))) (stale `StartPowerUp` Location))))
            (bind (_x _y) (`KismetMathLibrary.BreakVector2D` (stale `StartPowerUp` PowerUpRange)))
            (bind _output_get (set `self.ProximityPowerUpNormalize` (`KismetMathLibrary.MapRangeClamped` (`self.ProximityPowerUp`) (/ _x 2.0) (/ _y 2.0) 100.0)))
            (`KismetSystemLibrary.PrintString` (`KismetStringLibrary.Conv_DoubleToString` _output_get))))
        (else
          (set `self.ProximityPowerUp` (`KismetMathLibrary.VSize` (- (`self.K2_GetActorLocation` (`|GetArrayItem` _myfriend)) (`self.K2_GetActorLocation` (`|GetArrayItem` _myfriend 1)))))
          (set `self.ProximityPowerUpNormalize` (`KismetMathLibrary.MapRangeClamped` (`self.ProximityPowerUp`) _proximitypoweruprange_x _proximitypoweruprange_y 100.0)))))
    (:`then_1`
      ;[1 1 1] Set Location
      (`|ExecutionSequence`
        (:`then_0`
          (set `self.IdealLocation` (+ (`self.MidPoint`) (`self.IdealOffset`)))
          (set `self.CurrentLocation` (`self.K2_GetActorLocation`))
          (set `self.DeltaLocation` (- (`self.IdealLocation`) (`self.CurrentLocation`)))
          (set `self.MaxMovementThisFrame_PerAxis` (* (`self.BulbySpeedPerAxis`) (`GameplayStatics.GetWorldDeltaSeconds`)))
          (set `self.MovementThisFrameDueToCap` (0.0 0.0 0.0))
          (set `self.CurrentSpeedLimiter` (`self.BulbySpeedLimiter`))
          (`|ExecutionSequence`
            (:`then_0`
              (if (> _returnvalue _bulbydistancelimiter)
                (set `self.CapVector` (* (`KismetMathLibrary.Normal` _deltalocation) (- _returnvalue _bulbydistancelimiter)))
                (set `self.MovementThisFrameDueToCap` (+ (`self.CapVector`) (`self.MovementThisFrameDueToCap`)))
                (set `self.DeltaLocation` (- (`self.DeltaLocation`) (`self.CapVector`)))))
            (:`then_1`
              (`|ExecutionSequence`
                (:`then_0`
                  (if (> (`KismetMathLibrary.Abs` _deltalocation_x_13) _bulbydistancelimiterperaxis_x_7)
                    (set `self.MovementThisFrameDueToCap` (`KismetMathLibrary.MakeVector` (* (`KismetMathLibrary.SignOfFloat` _deltalocation_x_9) (- (`KismetMathLibrary.Abs` _deltalocation_x_11) _bulbydistancelimiterperaxis_x_6)) _movementthisframeduetocap_y_3 _movementthisframeduetocap_z_2))
                    (set `self.DeltaLocation` (`KismetMathLibrary.MakeVector` (+ _deltalocation_x_10 (`KismetMathLibrary.FClamp` _deltalocation_x_12 (* _bulbydistancelimiterperaxis_x_5 -1.0) _bulbydistancelimiterperaxis_x_5)) _deltalocation_y_9 _deltalocation_z_6))))
                (:`then_1`
                  (if (> (`KismetMathLibrary.Abs` _deltalocation_y_10) _bulbydistancelimiterperaxis_y_5)
                    (set `self.MovementThisFrameDueToCap` (`KismetMathLibrary.MakeVector` _movementthisframeduetocap_x_2 (* (`KismetMathLibrary.SignOfFloat` _deltalocation_y_5) (- (`KismetMathLibrary.Abs` _deltalocation_y_7) _bulbydistancelimiterperaxis_y_4)) _movementthisframeduetocap_z))
                    (set `self.DeltaLocation` (`KismetMathLibrary.MakeVector` _deltalocation_x_8 (+ _deltalocation_y_6 (`KismetMathLibrary.FClamp` _deltalocation_y_8 (* _bulbydistancelimiterperaxis_y_3 -1.0) _bulbydistancelimiterperaxis_y_3)) _deltalocation_z_5))))
                (:`then_2`
                  (if (> (`KismetMathLibrary.Abs` _deltalocation_z_7) _bulbydistancelimiterperaxis_z_3)
                    (set `self.MovementThisFrameDueToCap` (`KismetMathLibrary.MakeVector` _movementthisframeduetocap_x _movementthisframeduetocap_y (* (`KismetMathLibrary.SignOfFloat` _deltalocation_z) (- (`KismetMathLibrary.Abs` _deltalocation_z_3) _bulbydistancelimiterperaxis_z))))
                    (set `self.DeltaLocation` (`KismetMathLibrary.MakeVector` _deltalocation_x_4 _deltalocation_y_4 (+ _deltalocation_z_2 (`KismetMathLibrary.FClamp` _deltalocation_z_4 (* _bulbydistancelimiterperaxis_z_2 -1.0) _bulbydistancelimiterperaxis_z_2))))))))
            (:`then_2`
              (for _array_element (`self.SpeedAdjusters`)
                (bind (_distancerange _speedmultiplierrange) (break `/Game/Blueprints/Game/ChaseCamSpeedAdjustment` _array_element))
                (bind (_x_2 _y_2) (`KismetMathLibrary.BreakVector2D` _distancerange))
                (if (== _returnvalue_2 (`KismetMathLibrary.FClamp` _returnvalue_2 _x_2 _y_2))
                  (bind (_x_3 _y_3) (`KismetMathLibrary.BreakVector2D` _distancerange))
                  (bind (_x_4 _y_4) (`KismetMathLibrary.BreakVector2D` _speedmultiplierrange))
                  (set `self.CurrentSpeedLimiter` (* (`self.CurrentSpeedLimiter`) (`KismetMathLibrary.MapRangeUnclamped` (`KismetMathLibrary.VSize` (`self.DeltaLocation`)) _x_3 _y_3 _x_4 _y_4)))
                  (break))))
            (:`then_3`
              (set `self.DesiredMovementThisFrame` (`KismetMathLibrary.MakeVector` (`KismetMathLibrary.FMin` (`KismetMathLibrary.Abs` _deltalocation_x_14) (* _maxmovementthisframe_peraxis_x (`KismetMathLibrary.SignOfFloat` _deltalocation_x_15))) (`KismetMathLibrary.FMin` (`KismetMathLibrary.Abs` _deltalocation_y_11) (* _maxmovementthisframe_peraxis_y (`KismetMathLibrary.SignOfFloat` _deltalocation_y_12))) (`KismetMathLibrary.FMin` (`KismetMathLibrary.Abs` _deltalocation_z_8) (* _maxmovementthisframe_peraxis_z (`KismetMathLibrary.SignOfFloat` _deltalocation_z_9)))))
              (set `self.DesiredMovementThisFrame` (`KismetMathLibrary.ClampVectorSize` (`self.DesiredMovementThisFrame`) 0.0 (* (`self.CurrentSpeedLimiter`) (`GameplayStatics.GetWorldDeltaSeconds`)))))))
        (:`then_1`
          (`self.K2_SetActorLocation` (+ (`self.CurrentLocation`) (`self.DesiredMovementThisFrame`) (`self.MovementThisFrameDueToCap`))))
        (:`then_2`
          (`KismetMaterialLibrary.SetVectorParameterValue` "/Game/Materials/PlayerLoc_MP.PlayerLoc_MP" "PlayerXY" (make `LinearColor` (.x (`self.K2_GetActorLocation`)) (.y (`self.K2_GetActorLocation`)))))))
    (:`then_2`
      (`self.Damage Tick`))))

(fn `MidPointLocation`
  (locals (TotalLocation :type "Vector Structure"))
  (bind _myfriend (`self.MyFriend`))
  (for _array_element _myfriend
    (set `local.TotalLocation` (+ (`local.TotalLocation`) (`self.K2_GetActorLocation` _array_element))))
  (set `self.MidPoint` (/ (`local.TotalLocation`) (`KismetArrayLibrary.Array_Length` _myfriend))))

(fn `UserConstructionScript`
  (`SphereComponent.SetSphereRadius` (`self.SafeZone`) (`self.SafeZoneCurrentRadius`) true)
  (set `self.SafeZoneTransitionRadius` (`self.SafeZoneCurrentRadius`)))