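; Base enemy Character Blueprint that handles health, death and aggro, passing state to an AI Blackboard.
; Any damage lowers EnemyHealth, then either flags an attack and records the damage causer on the Blackboard, or destroys the actor when health runs out.
; A Bulby_BP entering the detection sphere sets the chase flag and the movement speed, with no logic to reset either.
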(event `self.ReceiveAnyDamage`
  (params (Damage :type "Float (single-precision)") (DamageType :type "DamageType Object Reference") (InstigatedBy :type "Controller Object Reference") (DamageCauser :type "Actor Object Reference"))
  (bind _returnvalue (`AIBlueprintHelperLibrary.GetBlackboard` null))
  ;[1 1 1] Damage and Health
  (bind _output_get (set `self.EnemyHealth` (- (`self.EnemyHealth`) Damage)))
  (`/Engine/EditorBlueprintResources/StandardMacros.CompareFloat` (`KismetMathLibrary.FClamp` _output_get 0.0 10000.0)
    (:`>`
      (`BlackboardComponent.SetValueAsBool` _returnvalue "AttackPlayer?" true)
      (`BlackboardComponent.SetValueAsObject` _returnvalue "AttackingPlayer" DamageCauser))
    (:`==`
      (`self.K2_DestroyActor` :!label _label))
    (:`<`
      (goto _label))))

(event `self.Sphere.OnComponentBeginOverlap`
  (params (OverlappedComponent :type "PrimitiveComponent Object Reference") (OtherActor :type "Actor Object Reference") (OtherComp :type "PrimitiveComponent Object Reference") (OtherBodyIndex :type Integer) (bFromSweep :type Boolean) (SweepResult :type "HitResult Structure (by ref)"))
  ;[1 1 1] Chase
  (cast `/Game/Blueprints/PlayableCharacters/Bulby_BP` OtherActor)
  (`BlackboardComponent.SetValueAsBool` (`AIBlueprintHelperLibrary.GetBlackboard` null) "Chase?" true)
  (set `CharacterMovementComponent.MaxWalkSpeed` 300.0 (`self.CharacterMovement`)))

(fn `UserConstructionScript`)